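; BP_BetterChat is the AkhiToolkit mod's BetterChat plugin, providing the ".at" chat command.
; BeginPlay registers the plugin with a localized hint text.
; ExecuteCommand switches on the split command parameter and returns an "[AkhiToolkit]" chat message carrying the first player controller's net ID.
; The help branch returns only placeholder "Null Command" text, while any other input points to ".at help".
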(event EventBeginPlay
  (bind _text_ (CallFunction|GetLocalizedText "BC_HELP_Hit"))
  (CallFunction|NewPlugin ".at" "AkhiToolkit" (Utilities|Struct|MakeST_Command ".at" "" (Utilities|String|ToString(Text) _text_))))

(fn ConstructionScript
  (|CallParentFunction))

(fn ExecuteCommand
  (params (Command%20Param :type String))
  (Utilities|FlowControl|Sequence
    (:then_0
      (switch string (.RightS (Utilities|String|Split Command%20Param " "))
        (:Default
          (LocalVariables|SetReturn%20Str " 
——> .at help"))
        (:help
          (LocalVariables|SetReturn%20Str "Null Command"))))
    (:then_1
      (return true true (Utilities|Struct|MakeS_ChatMessage "[AkhiToolkit]" (LocalVariables|GetReturn%20Str) (Class|AdvancedSessionsLibrary|GetUniqueNetID (Game|GetPlayerController 0))) false))))